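; BP_InwardCollapse is a Chaos field Blueprint that breaks and pushes geometry collections as soon as play begins.
; InCollapse applies a high external cluster strain through a box falloff field, sized and placed by the Box component with no falloff.
; It then applies a uniform linear velocity along fixed +Y, which is neither limited to the box nor aimed at its center.
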(event Custom|InCollapse
  (bind _fieldsystemcomponent (Variables|Field|GetFieldSystemComponent))
  (bind _box (Variables|Default|GetBox))
  (Class|FieldSystemComponent|ApplyPhysicsField _fieldsystemcomponent true "Field_ExternalClusterStrain" 0 (Field|SetBoxFalloff (Variables|Default|GetBoxFalloff) 5e+05 0.0 1.0 0.0 (Math|Transform|MakeTransform (Transformation|GetWorldLocation _box) "0, 0, 0" (Components|Box|GetScaledBoxExtent _box)) "Field_FallOff_None"))
  (Class|FieldSystemComponent|ApplyPhysicsField _fieldsystemcomponent true "Field_LinearVelocity" 0 (Field|SetUniformVector (Variables|Default|GetUniformVector) 1e+03 "0.000000,1.000000,0.000000")))

(event EventBeginPlay
  (CallFunction|InCollapse))

(fn ConstructionScript)