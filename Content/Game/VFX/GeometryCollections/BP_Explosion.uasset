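; BP_Explosion is a Chaos field actor that fractures nearby Geometry Collections and blows the pieces outward when play begins.
; On BeginPlay, Explode applies an external cluster strain through a radial falloff sized and centered on the Sphere component.
; It then applies a radial linear velocity from the same center, using a culling field to confine the push to that sphere.
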(event Custom|Explode
  (bind _fieldsystemcomponent (Variables|Field|GetFieldSystemComponent))
  (bind _radialfalloff (Variables|Default|GetRadialFalloff))
  (bind _sphere (Variables|Default|GetSphere))
  (bind _returnvalue (Components|Sphere|GetScaledSphereRadius _sphere))
  (bind _returnvalue_2 (Transformation|GetWorldLocation _sphere))
  (bind _returnvalue_3 (Field|SetRadialFalloff _radialfalloff 5e+06 0.0 1.0 0.0 _returnvalue _returnvalue_2 "Field_FallOff_None"))
  (Class|FieldSystemComponent|ApplyPhysicsField _fieldsystemcomponent true "Field_ExternalClusterStrain" 0 _returnvalue_3)
  (Class|FieldSystemComponent|ApplyPhysicsField _fieldsystemcomponent true "Field_LinearVelocity" 0 (Field|SetCullingField (Variables|Default|GetCullingField) _returnvalue_3 (Field|SetRadialVector (Variables|Default|GetRadialVector) 1e+03 (Transformation|GetWorldLocation (Variables|Default|GetSphere))) "Field_Culling_Outside")))

(event EventBeginPlay
  (CallFunction|Explode))

(fn ConstructionScript)